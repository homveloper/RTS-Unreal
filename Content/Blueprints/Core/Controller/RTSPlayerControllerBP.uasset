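; RTS player controller that moves the camera pawn from player axis input.
; On BeginPlay it casts the first player pawn to RTSCameraPawnBP and caches the reference.
; The MoveVertical and MoveHorizontal axes feed the pawn's FloatingPawnMovement as input vectors along world Y and X respectively.
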(event EventBeginPlay
  (Utilities|ReferenceCast) ; Should be first
)

(event Input|AxisEvents|InputAxisMoveHorizontal
  (params (AxisValue :type Float%20%28single-precision%29))
  (Class|PawnMovementComponent|AddInputVector (Variables|/Game/Blueprints/Core/Camera/RTSCameraPawnBP.RTSCameraPawnBP_C|GetFloatingPawnMovement (Variables|References|GetCameraPawnRef)) (Math|Vector|MakeVector AxisValue 0.0 0.0) false))

(event Input|AxisEvents|InputAxisMoveVertical
  (params (AxisValue :type Float%20%28single-precision%29))
  (Class|PawnMovementComponent|AddInputVector (Variables|/Game/Blueprints/Core/Camera/RTSCameraPawnBP.RTSCameraPawnBP_C|GetFloatingPawnMovement (Variables|References|GetCameraPawnRef)) (Math|Vector|MakeVector 0.0 AxisValue 0.0) false))

(fn ConstructionScript)